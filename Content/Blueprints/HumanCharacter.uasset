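; Player human character with Enhanced Input, health component, stamina-limited sprint toggle and weapon handling.
; Move input is stored as forward/right values, doubled while sprinting, as Tick drains or regenerates stamina.
; Overlapped weapons attach to the right-hand socket, feed the HUD widget and receive fire, secondary fire and reload input.
; Death and fire responses only print; debug keys apply damage or face the cursor through plane intersection.
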(event `self.ReceiveBeginPlay`
  (bind _returnvalue (pcsubsystem `EnhancedInputLocalPlayerSubsystem` (`GameplayStatics.GetPlayerController` 0)))
  ;[1 1 1] Begin Play
  (add `/Game/Blueprints/Components/BPC_Health.Death` (`self.BPC_Health`) (delegate `Death`))
  (`EnhancedInputSubsystemInterface.AddMappingContext` _returnvalue "/Game/Blueprints/Input/Movement/Movement.Movement" 0 (make `ModifyContextOptions` false true))
  (`EnhancedInputSubsystemInterface.AddMappingContext` _returnvalue "/Game/Blueprints/Input/Actions/Actions.Actions" 0 (make `ModifyContextOptions` false true))
  (bind _asplayer_controller (cast `PlayerController` (`self.GetController`)))
  (bind _returnvalue_2 (`|CreateWidget` "/Game/Blueprints/UI/HUD.HUD_C" _asplayer_controller null self (`self.BPC_Health`)))
  (bind _output_get (set `self.HUDInst` _returnvalue_2))
  (`WidgetComponent.SetWidget` (`self.HUD`) _output_get))

(event `Key|L`
  (params (Key :type "Key Structure"))
  (:`Pressed`
    (`/Game/Blueprints/Components/BPC_Health.Apply Damage` (`self.BPC_Health`) 2.0)))

(event `Death`
  (`KismetSystemLibrary.PrintString` "Hello we died"))

(event `EnhancedInput|/Game/Blueprints/Input/Movement/MoveUp`
  (params (ActionValue :type "Float (double-precision)") (ElapsedSeconds :type "Float (double-precision)") (TriggeredSeconds :type "Float (double-precision)") (InputAction :type "InputAction Object Reference" :default "/Game/Blueprints/Input/Movement/MoveUp.MoveUp"))
  ;[1 1 1] Movement
  (:`Triggered`
    (set `self.Input Forward` (* ActionValue (`KismetMathLibrary.SelectFloat` 2.0 1.0 (`self.Sprint?`))) :!label _label))
  (:`Completed`
    (goto _label)))

(event `EnhancedInput|/Game/Blueprints/Input/Movement/Sprint`
  (params (ActionValue :type Boolean) (ElapsedSeconds :type "Float (double-precision)") (TriggeredSeconds :type "Float (double-precision)") (InputAction :type "InputAction Object Reference" :default "/Game/Blueprints/Input/Movement/Sprint.Sprint"))
  ;[1 1 1] Sprinting
  (:`Started`
    (if (> (`self.Stamina`) 0.0)
      (set `self.Sprint?` (not (`self.Sprint?`))))))

(event `EnhancedInput|/Game/Blueprints/Input/Movement/MoveRight`
  (params (ActionValue :type "Float (double-precision)") (ElapsedSeconds :type "Float (double-precision)") (TriggeredSeconds :type "Float (double-precision)") (InputAction :type "InputAction Object Reference" :default "/Game/Blueprints/Input/Movement/MoveRight.MoveRight"))
  ;[1 1 1] Movement
  (:`Triggered`
    (set `self.Input Right` (* ActionValue (`KismetMathLibrary.SelectFloat` 2.0 1.0 (`self.Sprint?`))) :!label _label_2))
  (:`Completed`
    (goto _label_2)))

(event `Key|P`
  (params (Key :type "Key Structure"))
  (bind _returnvalue (`GameplayStatics.GetPlayerController` 0))
  (bind _returnvalue_2 (`self.K2_GetActorLocation`))
  (bind (_worldlocation _worlddirection) (`PlayerController.DeprojectMousePositionToWorld` _returnvalue))
  (bind (_t _intersection _returnvalue_3) (`KismetMathLibrary.LinePlaneIntersection` _worldlocation (+ _worldlocation (* _worlddirection (1000.0 1000.0 1000.0))) (`KismetMathLibrary.MakePlaneFromPointAndNormal` _returnvalue_2 (0.0 0.0 1.0))))
  ;[1 1 1] Mouse rotation
  (:`Pressed`
    (set `PlayerController.bShowMouseCursor` true _returnvalue)
    (if _returnvalue_3
      (`Controller.SetControlRotation` _returnvalue (`KismetMathLibrary.FindLookAtRotation` _returnvalue_2 _intersection)))))

(event `EnhancedInput|/Game/Blueprints/Input/Movement/RotateUp`
  (params (ActionValue :type "Float (double-precision)") (ElapsedSeconds :type "Float (double-precision)") (TriggeredSeconds :type "Float (double-precision)") (InputAction :type "InputAction Object Reference" :default "/Game/Blueprints/Input/Movement/RotateUp.RotateUp"))
  ;[1 1 1] Rotation
  (:`Triggered`
    (`self.AddControllerPitchInput` ActionValue)))

(event `EnhancedInput|/Game/Blueprints/Input/Movement/RotateRight`
  (params (ActionValue :type "Float (double-precision)") (ElapsedSeconds :type "Float (double-precision)") (TriggeredSeconds :type "Float (double-precision)") (InputAction :type "InputAction Object Reference" :default "/Game/Blueprints/Input/Movement/RotateRight.RotateRight"))
  ;[1 1 1] Rotation
  (:`Triggered`
    (`self.AddControllerYawInput` ActionValue)))

(event `EnhancedInput|/Game/Blueprints/Input/Actions/Fire1`
  (params (ActionValue :type Boolean) (ElapsedSeconds :type "Float (double-precision)") (TriggeredSeconds :type "Float (double-precision)") (InputAction :type "InputAction Object Reference" :default "/Game/Blueprints/Input/Actions/Fire1.Fire1"))
  (bind _currentweapon (`self.CurrentWeapon`))
  (:`Started`
    (`/Engine/EditorBlueprintResources/StandardMacros.IsValid` _currentweapon
      (:`Is Valid`
        (`/Game/Blueprints/Weapons/BP_Weapon.Event TriggerPull` _currentweapon))))
  (:`Completed`
    (`/Engine/EditorBlueprintResources/StandardMacros.IsValid` _currentweapon
      (:`Is Valid`
        (`/Game/Blueprints/Weapons/BP_Weapon.Event TriggerRelease` _currentweapon)))))

(event `EnhancedInput|/Game/Blueprints/Input/Actions/Fire2`
  (params (ActionValue :type Boolean) (ElapsedSeconds :type "Float (double-precision)") (TriggeredSeconds :type "Float (double-precision)") (InputAction :type "InputAction Object Reference" :default "/Game/Blueprints/Input/Actions/Fire2.Fire2"))
  (bind _currentweapon (`self.CurrentWeapon`))
  (:`Started`
    (`/Engine/EditorBlueprintResources/StandardMacros.IsValid` _currentweapon
      (:`Is Valid`
        (`/Game/Blueprints/Weapons/BP_Weapon.Fire2` _currentweapon))))
  (:`Completed`
    (`/Engine/EditorBlueprintResources/StandardMacros.IsValid` _currentweapon
      (:`Is Valid`
        (`/Game/Blueprints/Weapons/BP_Weapon.End Fire2` _currentweapon)))))

(event `self.ReceiveTick`
  (params (DeltaSeconds :type "Float (single-precision)"))
  ;[1 1 1] Event Tick
  (set `self.Delta Seconds` DeltaSeconds)
  (`self.HandleStamina`))

(event `EnhancedInput|/Game/Blueprints/Input/Actions/Reload`
  (params (ActionValue :type Boolean) (ElapsedSeconds :type "Float (double-precision)") (TriggeredSeconds :type "Float (double-precision)") (InputAction :type "InputAction Object Reference" :default "/Game/Blueprints/Input/Actions/Reload.Reload"))
  (bind _currentweapon (`self.CurrentWeapon`))
  (:`Started`
    (`/Engine/EditorBlueprintResources/StandardMacros.IsValid` _currentweapon
      (:`Is Valid`
        (`/Game/Blueprints/Weapons/BP_Weapon.Reload` _currentweapon)))))

(event `HandleFire`
  (`KismetSystemLibrary.PrintString` "Play FireAnim")
  (`KismetSystemLibrary.PrintString` "Change FiringStats")
  (`KismetSystemLibrary.PrintString` "Update Accuracy"))

(event `self.ReceiveActorBeginOverlap`
  (params (OtherActor :type "Actor Object Reference"))
  (bind _currentweapon (`self.CurrentWeapon`))
  ;[1 1 1] Collect Weapon
  (if (== (`GameplayStatics.GetObjectClass` OtherActor) "/Game/Blueprints/Weapons/BP_Weapon.BP_Weapon_C")
    (`self.AttachWeapon` OtherActor)
    (set `/Game/Blueprints/UI/HUD.Weapon` _currentweapon (`self.HUDInst`))
    (add `/Game/Blueprints/Weapons/BP_Weapon.Fire` _currentweapon (delegate `HandleFire`))))

(fn `AttachWeapon`
  (params (Weapon :type "Actor Object Reference"))
  (`SceneComponent.K2_AttachToComponent` (`Actor.RootComponent` Weapon) (`self.Mesh`) "RightHand" "SnapToTarget" "SnapToTarget" "KeepWorld" true)
  (bind _asbp_weapon (cast `/Game/Blueprints/Weapons/BP_Weapon` Weapon))
  (set `self.CurrentWeapon` _asbp_weapon)
  (`self.SetActorEnableCollision` _asbp_weapon false))

(fn `HandleStamina`
  (bind _stamina (`self.Stamina`))
  (bind _stamina_2 (`self.Stamina`))
  (if (`self.Sprint?`)
    (bind _output_get (set `self.Stamina` (`KismetMathLibrary.FClamp` (- _stamina_2 (* (`self.StaminaDrain`) (`self.Delta Seconds`))) 0.0 _stamina_2)))
    (if (<= _output_get 0.0)
      (set `self.Sprint?` false))
    (else
      (set `self.Stamina` (`KismetMathLibrary.FClamp` (+ (* (`self.Delta Seconds`) (`self.StaminaRegen`)) _stamina) _stamina (`self.StaminaMax`))))))

(fn `UserConstructionScript`)
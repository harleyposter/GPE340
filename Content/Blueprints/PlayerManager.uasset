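; PlayerManager runs the player's lifecycle and end-of-game flow: spawning, limited-life respawns, and win or lose.
; It spawns a HumanCharacter at RespawnSpot with configured stats, weapon and colors, possesses it and binds to its health component's death event.
; Each death respawns and rebinds while Lives remain, otherwise triggers Lose.
; Win and Lose show their screen widgets and quit after a delay, with Win also unpossessing the player.
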(event `self.ReceiveBeginPlay`
  ;[1 1 1] Initializing
  (bind _returnvalue (`|SpawnActorFromClass` "/Game/Blueprints/HumanCharacter.HumanCharacter_C" (`KismetMathLibrary.MakeTransform` (`SceneComponent.K2_GetComponentLocation` (`self.RespawnSpot`))) "AdjustIfPossibleButAlwaysSpawn" "MultiplyWithRoot" null (`self.Health`) (`self.AccuracyOffset`) (`self.Stamina Max`) (`self.Stamina Regen`) (`self.Stamina Drain`) (`self.WeaponType`) "/Game/Art/Materials/BlueMain.BlueMain" "/Game/Art/Materials/BlueJoints.BlueJoints" null))
  (bind _output_get (set `self.Player` _returnvalue))
  (`Controller.Possess` (`GameplayStatics.GetPlayerController` 0) _output_get)
  (add `/Game/Blueprints/Components/BPC_Health.Death` (`/Game/Blueprints/HumanCharacter.BPC_Health` (`self.Player`)) (delegate `PlayerDeath`)))

(event `PlayerDeath`
  (bind _lives (`self.Lives`))
  ;[1 1 1] Respawn
  (if (>= _lives 1)
    (`/Engine/EditorBlueprintResources/StandardMacros.DecrementInt` _lives
      (:`  `
        (bind _returnvalue (`|SpawnActorFromClass` "/Game/Blueprints/HumanCharacter.HumanCharacter_C" (`KismetMathLibrary.MakeTransform` (`SceneComponent.K2_GetComponentLocation` (`self.RespawnSpot`))) "AdjustIfPossibleButAlwaysSpawn" "MultiplyWithRoot" null (`self.Health`) (`self.AccuracyOffset`) (`self.Stamina Max`) (`self.Stamina Regen`) (`self.Stamina Drain`) (`self.WeaponType`) "/Game/Art/Materials/BlueMain.BlueMain" "/Game/Art/Materials/BlueJoints.BlueJoints" null))
        (`Controller.Possess` (`Pawn.GetController` (`self.Player`)) _returnvalue)
        (set `self.Player` _returnvalue)
        (add `/Game/Blueprints/Components/BPC_Health.Death` (`/Game/Blueprints/HumanCharacter.BPC_Health` (`self.Player`)) (delegate `PlayerDeath`))))
    (else
      (`self.Lose`))))

(event `Win`
  (bind _returnvalue (`GameplayStatics.GetPlayerController` 0))
  (bind _player (`self.Player`))
  ;[1 1 1] Win and Lose
  (bind _returnvalue_2 (`|CreateWidget` "/Game/Blueprints/UI/WinScreen.WinScreen_C" _returnvalue self))
  (`UserWidget.AddToViewport` _returnvalue_2 0)
  (`Controller.UnPossess` _returnvalue)
  (set `/Game/Blueprints/HumanCharacter.Input Forward` 0.0 _player)
  (set `/Game/Blueprints/HumanCharacter.Input Right` 0.0 _player)
  (`KismetSystemLibrary.Delay` 10.0)
  (`KismetSystemLibrary.QuitGame` null "Quit"))

(event `Lose`
  ;[1 1 1] Win and Lose
  (bind _returnvalue (`|CreateWidget` "/Game/Blueprints/UI/LoseScreen.LoseScreen_C" (`GameplayStatics.GetPlayerController` 0) self))
  (`UserWidget.AddToViewport` _returnvalue 0)
  (`KismetSystemLibrary.Delay` 10.0)
  (`KismetSystemLibrary.QuitGame` null "Quit"))

(fn `UserConstructionScript`)
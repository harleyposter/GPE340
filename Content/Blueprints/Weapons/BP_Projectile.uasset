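; BP_Projectile is a weapon projectile that flies forward and damages actors it overlaps.
; On BeginPlay it feeds its Velocity variable into the ProjectileMovement component along the actor's forward vector.
; On overlap with an actor that has a BPC_Health component, it applies Damage through that component and destroys itself, ignoring actors without one.
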(event `self.ReceiveBeginPlay`
  (bind _projectilemovement (`self.ProjectileMovement`))
  (bind _velocity (`self.Velocity`))
  (set `ProjectileMovementComponent.InitialSpeed` _velocity _projectilemovement)
  (set `MovementComponent.Velocity` (* (`KismetMathLibrary.GetForwardVector` (`self.K2_GetActorRotation`)) _velocity) _projectilemovement))

(event `self.ReceiveActorBeginOverlap`
  (params (OtherActor :type "Actor Object Reference"))
  (bind _returnvalue (`self.GetComponentByClass` OtherActor "/Game/Blueprints/Components/BPC_Health.BPC_Health_C"))
  (if (`KismetSystemLibrary.IsValid` _returnvalue)
    (`/Game/Blueprints/Components/BPC_Health.Apply Damage` _returnvalue (`self.Damage`))
    (`self.K2_DestroyActor`)))

(fn `UserConstructionScript`)
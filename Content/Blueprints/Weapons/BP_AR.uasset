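; BP_AR is an assault rifle Blueprint whose ShootSecondary function fires a burst of up to three shots with no delay between them.
; Each shot calls Fire, line-traces from FirePoint toward Target out to Range with debug drawing, and damages any hit actor's BPC_Health.
; The loop decrements Rounds between shots and stops when ShotCount hits three or ammo runs out.
; ShotCount is not reset in this graph.
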(fn `ShootSecondary`
  (returns (Target :type "Vector Structure"))
  (locals (`Firing End Dir` :type "Vector Structure") (ShotCount :type Integer))
  (bind _shotcount (`local.ShotCount`))
  (bind _rounds (`self.Rounds`))
  (bind _returnvalue_location (`KismetMathLibrary.BreakTransform` (`SceneComponent.K2_GetComponentToWorld` (`self.Fire Point`))))
  (bind _returnvalue (+ _returnvalue_location (* (`KismetMathLibrary.GetDirectionUnitVector` _returnvalue_location (`SceneComponent.K2_GetComponentLocation` (`self.Target`))) (`self.Range`))))
  (`self.Fire` :!label _label)
  (bind _output_get (set `local.Firing End Dir` _returnvalue))
  (bind (_outhit _returnvalue_2) (`KismetSystemLibrary.LineTraceSingleForObjects` :`Start` _returnvalue_location :`End` _returnvalue :`ObjectTypes` (`|MakeArray` "ObjectTypeQuery1" "ObjectTypeQuery2" "ObjectTypeQuery3" :!type "EObjectTypeQuery Enum") :`DrawDebugType` "ForDuration"))
  (if _returnvalue_2
    (bind _returnvalue_3 (`self.GetComponentByClass` (`.HitActor` (`GameplayStatics.BreakHitResult` _outhit)) "/Game/Blueprints/Components/BPC_Health.BPC_Health_C"))
    (if (`KismetSystemLibrary.IsValid` _returnvalue_3)
      (`/Game/Blueprints/Components/BPC_Health.Apply Damage` _returnvalue_3 (`self.Damage`))))
  (set `local.ShotCount` (+ _shotcount 1))
  (if (== _shotcount 3)
    _
    (elif (<= _rounds 0)
      _
      (else
        (`/Engine/EditorBlueprintResources/StandardMacros.DecrementInt` _rounds
          (:`  `
            (goto _label))))))
  (return _output_get))

(fn `UserConstructionScript`
  (`parent.UserConstructionScript`))
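; Weapon actor with automatic primary and secondary fire that share rounds, fire rate and reload.
; Trigger events set autofire flags that Tick polls, with delays gating each shot and an empty magazine starting a timed reload from reserve ammo.
; Primary fire line-traces and damages BPC_Health, while secondary launches BP_Projectile.
; Both aim from FirePoint toward a Target with accuracy-based random spread, then spawn a Niagara effect and play audio.
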(event `self.ReceiveBeginPlay`)

(event `Event TriggerPull`
  ;[1 1 1] Assign Dispatchers
  (`self.Autofire1Begin`))

(event `Event TriggerRelease`
  ;[1 1 1] Assign Dispatchers
  (`self.Autofire1End`))

(event `Fire1`
  ;[1 1 1] Primary Fire
  (set `self.Firing1?` true)
  (if (>= (`self.Rounds`) 1)
    (if (`self.CanFire1?`)
      (set `self.CanFire1?` false)
      (bind _firingtarget (`self.ShootPrimary`))
      (`self.SpawnParticle` (`SceneComponent.K2_GetComponentLocation` (`self.Fire Point`)) _firingtarget)
      (`AudioComponent.Play` (`self.Audio`) 0.0)
      (`/Engine/EditorBlueprintResources/StandardMacros.DecrementInt` (`self.Rounds`)
        (:`  `
          (`KismetSystemLibrary.Delay` (/ 1.0 (`self.FireRate`)))
          (set `self.CanFire1?` true))))
    (else
      (`self.Reload`))))

(event `Event Trigger2Pull`
  ;[1 1 1] Assign Dispatchers
  (`self.Autofire2Begin`))

(event `EventTrigger2Release`
  ;[1 1 1] Assign Dispatchers
  (`self.Autofire2End`))

(event `End Fire1`
  ;[1 1 1] Primary Fire
  (set `self.Firing1?` false))

(event `Autofire1Begin`
  ;[1 1 1] Primary Fire
  (set `self.Autofire1?` true))

(event `self.ReceiveTick`
  (params (DeltaSeconds :type "Float (single-precision)"))
  ;[1 1 1] Event Tick
  (`|ExecutionSequence`
    (:`then_0`
      (if (`self.Autofire1?`)
        (`self.Fire1`)))
    (:`then_1`
      (if (`self.Autofire2?`)
        (`self.Fire2`)))))

(event `Autofire1End`
  ;[1 1 1] Primary Fire
  (set `self.Autofire1?` false)
  (`self.End Fire1`))

(event `Fire2`
  ;[1 1 1] Secondary Fire
  (set `self.Firing2?` true)
  (if (>= (`self.Rounds`) 1)
    (if (`self.CanFire2?`)
      (set `self.CanFire2?` false)
      (bind _target (`self.ShootSecondary`))
      (`self.SpawnParticle` (`SceneComponent.K2_GetComponentLocation` (`self.Fire Point`)) _target)
      (`AudioComponent.Play` (`self.Audio`) 0.0)
      (`/Engine/EditorBlueprintResources/StandardMacros.DecrementInt` (`self.Rounds`)
        (:`  `
          (`KismetSystemLibrary.Delay` (/ 1.0 (`self.FireRate`)))
          (set `self.CanFire2?` true))))
    (else
      (`self.Reload`))))

(event `On Equipped`
  (params (Target :type "SceneComponent Object Reference"))
  (set `self.Target` Target))

(event `On Unequipped`
  (`self.K2_DestroyActor`))

(event `End Fire2`
  ;[1 1 1] Secondary Fire
  (set `self.Firing2?` false))

(event `Autofire2Begin`
  ;[1 1 1] Secondary Fire
  (set `self.Autofire2?` true))

(event `Autofire2End`
  ;[1 1 1] Secondary Fire
  (set `self.Autofire2?` false)
  (`self.End Fire2`))

(event `Reload`
  ;[1 1 1] Reload
  (if (and (>= (`self.Ammo`) 1) (`self.CanReload?`) (< (`self.Rounds`) (`self.RoundsMax`)))
    (set `self.Reloading?` true)
    (set `self.CanReload?` false)
    (set `self.CanFire1?` false)
    (set `self.CanFire2?` false)
    (`KismetSystemLibrary.Delay` (`self.ReloadTime`))
    (`self.HandleReload`)
    (set `self.CanFire1?` true)
    (set `self.CanReload?` true)
    (set `self.CanFire2?` true)
    (set `self.Reloading?` false)))

(fn `Calculate Accuracy`
  (returns (AccuracyOffset :type "Vector Structure"))
  (bind _returnvalue_location (`KismetMathLibrary.BreakTransform` (`SceneComponent.K2_GetComponentToWorld` (`self.Fire Point`))))
  (bind _returnvalue (- (`self.Accuracy`) 100.0))
  (bind _returnvalue_2 (/ 1000.0 (`self.Range`)))
  (bind _returnvalue_3 (`KismetMathLibrary.Abs` (* (`KismetMathLibrary.FClamp` _returnvalue _returnvalue 0.0) 3.0)))
  (bind _returnvalue_4 (`KismetMathLibrary.RandomFloatInRange` (* (* _returnvalue_3 -1.0) _returnvalue_2) (* _returnvalue_3 _returnvalue_2)))
  (return (`KismetMathLibrary.RotateAngleAxis` (`KismetMathLibrary.MakeVector` _returnvalue_4 _returnvalue_4 _returnvalue_4) (`KismetMathLibrary.RandomFloatInRange` 0.0 360.0) (`KismetMathLibrary.GetDirectionUnitVector` _returnvalue_location (`SceneComponent.K2_GetComponentLocation` (`self.Target`))))))

(fn `HandleReload`
  (locals (RoundsLeft :type Integer))
  (bind _ammo (`self.Ammo`))
  (set `local.RoundsLeft` (`self.Rounds`))
  (set `self.Rounds` (`KismetMathLibrary.Clamp` (+ (`self.Ammo`) (`self.Rounds`)) 0 (`self.RoundsMax`)))
  (set `self.Ammo` (`KismetMathLibrary.Clamp` (- _ammo (- (`self.RoundsMax`) (`local.RoundsLeft`))) 0 _ammo)))

(fn `ShootPrimary`
  (returns (FiringTarget :type "Vector Structure"))
  (locals (FiringEndDir :type "Vector Structure"))
  (bind _returnvalue_location (`KismetMathLibrary.BreakTransform` (`SceneComponent.K2_GetComponentToWorld` (`self.Fire Point`))))
  (`self.Fire`)
  (bind _output_get (set `local.FiringEndDir` (+ _returnvalue_location (* (`KismetMathLibrary.GetDirectionUnitVector` _returnvalue_location (+ (`SceneComponent.K2_GetComponentLocation` (`self.Target`)) (`self.Calculate Accuracy`))) (`self.Range`)))))
  (bind (_outhit _returnvalue) (`KismetSystemLibrary.LineTraceSingleForObjects` _returnvalue_location _output_get (`|MakeArray` "ObjectTypeQuery1" "ObjectTypeQuery2" "ObjectTypeQuery3" :!type "EObjectTypeQuery Enum")))
  (if _returnvalue
    (bind _returnvalue_2 (`self.GetComponentByClass` (`.HitActor` (`GameplayStatics.BreakHitResult` _outhit)) "/Game/Blueprints/Components/BPC_Health.BPC_Health_C"))
    (if (`KismetSystemLibrary.IsValid` _returnvalue_2)
      (`/Game/Blueprints/Components/BPC_Health.Apply Damage` _returnvalue_2 (`self.Damage`))
      (return (`.TraceEnd` (`GameplayStatics.BreakHitResult` _outhit))))
    (else
      (return (`.TraceEnd` (`GameplayStatics.BreakHitResult` _outhit))))))

(fn `ShootSecondary`
  (returns (Target :type "Vector Structure"))
  (locals (FiringEndDir :type "Vector Structure"))
  (bind _returnvalue_location (`KismetMathLibrary.BreakTransform` (`SceneComponent.K2_GetComponentToWorld` (`self.Fire Point`))))
  (bind _returnvalue_location_2 (`KismetMathLibrary.BreakTransform` (`SceneComponent.K2_GetComponentToWorld` (`self.Fire Point`))))
  (bind _returnvalue (+ _returnvalue_location (* (`KismetMathLibrary.GetDirectionUnitVector` _returnvalue_location (+ (`SceneComponent.K2_GetComponentLocation` (`self.Target`)) (`self.Calculate Accuracy`))) (`self.Range`))))
  (`self.Fire`)
  (`|SpawnActorFromClass` "/Game/Blueprints/Weapons/BP_Projectile.BP_Projectile_C" (`KismetMathLibrary.MakeTransform` _returnvalue_location_2 (`KismetMathLibrary.FindLookAtRotation` _returnvalue_location_2 _returnvalue) (0.5 0.5 0.5)) "Undefined" "MultiplyWithRoot" null (`self.Damage`) (* (`self.Range`) 10.0) null)
  (return _returnvalue))

(fn `SpawnParticle`
  (params (Start :type "Vector Structure (by ref)") (Target :type "Vector Structure (by ref)"))
  (bind _returnvalue (`NiagaraFunctionLibrary.SpawnSystemAtLocation` "/Game/Blueprints/Particles/FireWeapon.FireWeapon" Start (`KismetMathLibrary.FindLookAtRotation` Start Target) (1.0 1.0 1.0) true false))
  (`NiagaraComponent.SetVariableVec3` _returnvalue "Range" (`KismetMathLibrary.MakeVector` (`self.Range`)))
  (`ActorComponent.Activate` _returnvalue false))

(fn `UserConstructionScript`)
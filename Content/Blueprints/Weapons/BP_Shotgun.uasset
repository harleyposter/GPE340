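; BP_Shotgun is a shotgun weapon that overrides an inherited primary fire event to shoot a burst of pellets per round.
; Each pellet calls ShootPrimary and feeds its result to SpawnParticle as the target of an effect from the fire point.
; A shot plays audio, spends one round and gates refire with a delay derived from FireRate.
; Firing without a round triggers Reload.
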(event `self.Fire1`
  ;[1 1 1] Fire 1 Override
  (set `self.Firing1?` true)
  (if (>= (`self.Rounds`) 1)
    (if (`self.CanFire1?`)
      (set `self.CanFire1?` false)
      (for _ (range 10)
        (bind _firingtarget (`self.ShootPrimary`))
        (`self.SpawnParticle` (`SceneComponent.K2_GetComponentLocation` (`self.Fire Point`)) _firingtarget))
      (`AudioComponent.Play` (`self.Audio`) 0.0)
      (`/Engine/EditorBlueprintResources/StandardMacros.DecrementInt` (`self.Rounds`)
        (:`  `
          (`KismetSystemLibrary.Delay` (/ 1.0 (`self.FireRate`)))
          (set `self.CanFire1?` true))))
    (else
      (`self.Reload`))))

(fn `UserConstructionScript`
  (`parent.UserConstructionScript`))
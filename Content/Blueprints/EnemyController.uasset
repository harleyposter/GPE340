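; AI controller that patrols a possessed HumanCharacter through a looping list of target points.
; It computes a synchronous navigation path to each point, draws debug traces, and walks the path with chained AI MoveTo calls, treating failure like success.
; It sets the character's forward input during moves and pauses briefly between targets.
; Tick yaws the pawn toward the current waypoint until Stop is set at the first path's end; nothing here clears it.
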(event `self.ReceivePossess`
  (params (PossessedPawn :type "Pawn Object Reference"))
  (bind _ashuman_character (cast `/Game/Blueprints/HumanCharacter` (`self.In Pawn`)))
  (set `self.As Human Character` _ashuman_character)
  (`self.Patrol`))

(event `Patrol`
  (bind _target_points (`self.Target Points`))
  (bind _point_id (`self.Point ID`))
  (if (>= _point_id (`KismetArrayLibrary.Array_Length` _target_points))
    (set `self.Point ID` 0))
  (`self.Find Path` (`self.K2_GetActorLocation` (`|GetArrayItem` _target_points _point_id))))

(event `Find Path`
  (params (`Target Point` :type "Vector Structure"))
  (bind _outactors (`GameplayStatics.GetAllActorsOfClass` "/Script/NavigationSystem.NavMeshBoundsVolume"))
  (bind _returnvalue (`NavigationSystemV1.FindPathToLocationSynchronously` (`self.K2_GetActorLocation` (`self.In Pawn`)) `Target Point` (`|GetArrayItem` _outactors) null))
  (bind _output_get (set `self.Path Points` (`NavigationPath.PathPoints` _returnvalue)))
  (for _array_element _output_get
    (`KismetSystemLibrary.LineTraceSingle` :`Start` _array_element :`End` (+ _array_element (0.0 0.0 100.0)) :`TraceChannel` "TraceTypeQuery1" :`DrawDebugType` "ForDuration"))
  (`self.Go To` (`|GetArrayItem` _output_get)))

(event `Go To`
  (params (`Target Point` :type "Vector Structure"))
  (bind _path_points (`self.Path Points`))
  (set `self.Target Point` `Target Point`)
  (`KismetSystemLibrary.LineTraceSingle` :`Start` `Target Point` :`End` (+ `Target Point` (0.0 0.0 100.0)) :`TraceChannel` "TraceTypeQuery1" :`DrawDebugType` "ForDuration")
  (`|AIMoveTo` (`self.K2_GetPawn`) `Target Point` null 100.0 true
    (:`then`
      (set `/Game/Blueprints/HumanCharacter.Input Forward` 1.0 (`self.As Human Character`)))
    (:`OnSuccess`
      (bind _result (`/Engine/EditorBlueprintResources/StandardMacros.IncrementInt` (`self.Path ID`) :!label _label)
        (:`  `
          (set `/Game/Blueprints/HumanCharacter.Input Forward` 0.0 (`self.As Human Character`))
          (if (> (`KismetArrayLibrary.Array_Length` _path_points) _result)
            (bind _output (`|GetArrayItem` _path_points _result))
            (`KismetSystemLibrary.PrintString` (`KismetStringLibrary.Conv_VectorToString` _output))
            (`self.Go To` _output)
            (else
              (set `self.Stop` true)
              (`/Engine/EditorBlueprintResources/StandardMacros.IncrementInt` (`self.Point ID`)
                (:`  `
                  (set `self.Path ID` 0)
                  (`KismetSystemLibrary.Delay` 1.0)
                  (`self.Patrol`))))))))
    (:`OnFail`
      (goto _label))))

(event `self.ReceiveTick`
  (params (DeltaSeconds :type "Float (single-precision)"))
  (bind _in_pawn (`self.In Pawn`))
  (bind (_returnvalue_roll _returnvalue_pitch) (`KismetMathLibrary.BreakRotator` (`self.K2_GetActorRotation` _in_pawn)))
  (bind (_returnvalue_roll_2 _returnvalue_pitch_2 _returnvalue_yaw) (`KismetMathLibrary.BreakRotator` (`KismetMathLibrary.FindLookAtRotation` (`self.K2_GetActorLocation` _in_pawn) (`self.Target Point`))))
  (if (not (`self.Stop`))
    (`self.K2_SetActorRotation` _in_pawn (`KismetMathLibrary.MakeRotator` _returnvalue_roll _returnvalue_pitch _returnvalue_yaw) false)))

(fn `UserConstructionScript`)
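; BPC_DelayedDeath is an actor component that destroys its owner a short, fixed time after that owner dies.
; On BeginPlay it looks up the owner's BPC_Health component and, if one exists, binds to its Death event.
; When that event fires, it waits five seconds and then destroys the owning actor.
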(event `self.ReceiveBeginPlay`
  (bind _returnvalue (`Actor.GetComponentByClass` (`self.GetOwner`) "/Game/Blueprints/Components/BPC_Health.BPC_Health_C"))
  (`parent.ReceiveBeginPlay`)
  (if (`KismetSystemLibrary.IsValid` _returnvalue)
    (add `/Game/Blueprints/Components/BPC_Health.Death` _returnvalue (delegate `self.Death Action`))))

(event `self.Death Action`
  (`KismetSystemLibrary.Delay` 5.0)
  (`Actor.K2_DestroyActor` (`self.GetOwner`)))
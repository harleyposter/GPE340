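; BPC_RespawnOnDeath is an actor component that respawns its owner after death.
; On BeginPlay it looks for a BPC_Health component on the owner and, if one exists, binds to its death event.
; On death it prints a debug message, waits a fixed delay, then spawns a new actor of the owner's class at the owner's transform.
; It does not destroy the original actor itself.
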(event `self.ReceiveBeginPlay`
  (bind _returnvalue (`Actor.GetComponentByClass` (`self.GetOwner`) "/Game/Blueprints/Components/BPC_Health.BPC_Health_C"))
  (`parent.ReceiveBeginPlay`)
  (if (`KismetSystemLibrary.IsValid` _returnvalue)
    (add `/Game/Blueprints/Components/BPC_Health.Death` _returnvalue (delegate `self.Death Action`))))

(event `self.Death Action`
  (bind _returnvalue (`self.GetOwner`))
  (`KismetSystemLibrary.PrintString` "Dead, Respawning")
  (`KismetSystemLibrary.Delay` 5.0)
  (`|SpawnActorFromClass` (`GameplayStatics.GetObjectClass` _returnvalue) (`Actor.GetTransform` _returnvalue) "Undefined" "MultiplyWithRoot" null null))
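; BPC_Health is a health component that tracks Health and handles damage, healing and death.
; ApplyDamage lowers Health with a floor of zero, plays SoundToPlay, then runs HandleDeath.
; ApplyHeal raises Health up to HealthMax.
; HandleDeath sets a Dead flag and calls Death once when Health reaches zero, with the flag blocking repeat calls.
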(event `Apply Damage`
  (params (`Damage Amount` :type "Float (double-precision)"))
  (bind _health (`self.Health`))
  (set `self.Health` (`KismetMathLibrary.FClamp` (- _health `Damage Amount`) 0.0 _health))
  (`AudioComponent.Play` (`self.SoundToPlay`) 0.0)
  (`self.Handle Death`))

(event `Apply Heal`
  (params (`Heal Amount` :type "Float (double-precision)"))
  (set `self.Health` (`KismetMathLibrary.FClamp` (+ `Heal Amount` (`self.Health`)) (`self.Health`) (`self.HealthMax`))))

(event `Handle Death`
  (if (and (<= (`self.Health`) 0.0) (not (`self.Dead?`)))
    (set `self.Dead?` true)
    (`self.Death`)))
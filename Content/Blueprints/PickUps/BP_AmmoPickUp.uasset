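; Ammo pickup that refills the player's current weapon.
; BeginPlay, overlap and Tick defer to the parent class; PickupAction runs only when the player holds a valid weapon.
; It fills Rounds to RoundsMax and adds a quarter of AmmoMax to Ammo, clamped to that maximum.
; The actor then hides, disables collision and destroys itself after a short delay.
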(event `self.ReceiveBeginPlay`
  (`parent.ReceiveBeginPlay`))

(event `self.ReceiveActorBeginOverlap`
  (params (OtherActor :type "Actor Object Reference"))
  (`parent.ReceiveActorBeginOverlap` OtherActor))

(event `self.ReceiveTick`
  (params (DeltaSeconds :type "Float (single-precision)"))
  (`parent.ReceiveTick` DeltaSeconds))

(event `self.Pickup Action`
  (bind _currentweapon (`/Game/Blueprints/HumanCharacter.CurrentWeapon` (`self.Player`)))
  (bind _ammomax (`/Game/Blueprints/Weapons/BP_Weapon.AmmoMax` _currentweapon))
  (`/Engine/EditorBlueprintResources/StandardMacros.IsValid` _currentweapon
    (:`Is Valid`
      (set `/Game/Blueprints/Weapons/BP_Weapon.Rounds` (`/Game/Blueprints/Weapons/BP_Weapon.RoundsMax` _currentweapon) _currentweapon)
      (set `/Game/Blueprints/Weapons/BP_Weapon.Ammo` (`KismetMathLibrary.Clamp` (+ (`/Game/Blueprints/Weapons/BP_Weapon.Ammo` _currentweapon) (* (`KismetMathLibrary.Conv_IntToDouble` _ammomax) 0.25)) 0 _ammomax) _currentweapon)
      (`self.SetActorHiddenInGame` true)
      (`self.SetActorEnableCollision` false)
      (`KismetSystemLibrary.Delay` 2.0)
      (`self.K2_DestroyActor`))))

(fn `UserConstructionScript`)
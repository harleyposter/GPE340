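; BP_HealPickUp is a health pickup that heals the player when collected.
; Its PickupAction event applies a fixed heal through the player's BPCHealth component.
; It then hides the actor and disables its collision, destroying it after a short delay.
; Overlap detection is not handled here, as its own BeginPlay, overlap and Tick events are disabled stubs.
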(event `self.Pickup Action`
  (`/Game/Blueprints/Components/BPC_Health.Apply Heal` (`/Game/Blueprints/HumanCharacter.BPC_Health` (`self.Player`)) 20.0)
  (`self.SetActorHiddenInGame` true)
  (`self.SetActorEnableCollision` false)
  (`KismetSystemLibrary.Delay` 2.0)
  (`self.K2_DestroyActor`))

(fn `UserConstructionScript`
  (`parent.UserConstructionScript`))
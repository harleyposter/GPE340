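; MyGameMode is a game mode Blueprint that controls audio volume for Master, SFX and Music channels.
; Each channel has a custom event that overrides its sound class volume through a dedicated sound mix, pushes that mix, then stores the value in a variable.
; It holds no other logic: BeginPlay, Tick and the construction script are empty.
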(event `Set Master Volume`
  (params (Volume :type "Float (single-precision)"))
  ;[1 1 1] Change Volume
  (`GameplayStatics.SetSoundMixClassOverride` "/Game/Blueprints/Sound/MasterSoundMix.MasterSoundMix" "/Game/Blueprints/Sound/MasterSoundClass.MasterSoundClass" Volume)
  (`GameplayStatics.PushSoundMixModifier` "/Game/Blueprints/Sound/MasterSoundMix.MasterSoundMix")
  (set `self.MasterVolume` Volume))

(event `Set SFX Volume`
  (params (Volume :type "Float (single-precision)"))
  ;[1 1 1] Change Volume
  (`GameplayStatics.SetSoundMixClassOverride` "/Game/Blueprints/Sound/SFXSoundMix.SFXSoundMix" "/Game/Blueprints/Sound/SFXSoundClass.SFXSoundClass" Volume)
  (`GameplayStatics.PushSoundMixModifier` "/Game/Blueprints/Sound/SFXSoundMix.SFXSoundMix")
  (set `self.SFXVolume` Volume))

(event `Set Music Volume`
  (params (Volume :type "Float (single-precision)"))
  ;[1 1 1] Change Volume
  (`GameplayStatics.SetSoundMixClassOverride` "/Game/Blueprints/Sound/MusicSoundMix.MusicSoundMix" "/Game/Blueprints/Sound/MusicSoundClass.MusicSoundClass" Volume)
  (`GameplayStatics.PushSoundMixModifier` "/Game/Blueprints/Sound/MusicSoundMix.MusicSoundMix")
  (set `self.MusicVolume` Volume))

(fn `UserConstructionScript`)
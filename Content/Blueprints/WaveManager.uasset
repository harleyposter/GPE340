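; Wave manager that runs timed enemy waves and calls Win on every PlayerManager once the final wave is cleared.
; SpawnWave greedily spends DifficultyPoints from Bosses down to Basics, placing enemies at random points in SpawnAreas boxes.
; Each enemy gets a spawned controller carrying points and weighted item drops.
; Defeats refund points into the budget, and clearing a wave adds a wave-scaled bonus before the next spawn.
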(event `self.ReceiveBeginPlay`
  (`KismetSystemLibrary.Delay` 3.0)
  (`self.SpawnWave`))

(event `ProgressWave`
  ;[1 1 1] Progress Wave
  (if (<= (`self.EnemiesLeft`) 0)
    (if (>= (`self.CurrentWave`) (`self.WaveCount`))
      (`KismetSystemLibrary.Delay` 5.0)
      (bind _outactors (`GameplayStatics.GetAllActorsOfClass` "/Game/Blueprints/PlayerManager.PlayerManager_C"))
      (for _array_element _outactors
        (`/Game/Blueprints/PlayerManager.Win` _array_element))
      (else
        (`KismetSystemLibrary.Delay` 5.0)
        (set `self.DifficultyPoints` (+ (`self.DifficultyPoints`) (* (`self.CurrentWave`) 2)))
        (`self.SpawnWave`)))))

(event `EnemyDefeated`
  (params (Enemy :type "/Game/Blueprints/EnemyController Object Reference"))
  (set `self.DifficultyPoints` (+ (`self.DifficultyPoints`) (`/Game/Blueprints/EnemyController.Points` Enemy)))
  (`/Engine/EditorBlueprintResources/StandardMacros.DecrementInt` (`self.EnemiesLeft`)
    (:`  `
      (`self.ProgressWave`))))

(event `HandleSpawn`
  (params (EnemyController :type "/Game/Blueprints/EnemyController Object Reference"))
  (add `/Game/Blueprints/EnemyController.EnemyDefeated` EnemyController (delegate `EnemyDefeated`)))

(fn `GetRandomSpawn`
  (returns (ReturnValue :type "Vector Structure"))
  (bind _spawnareas (`self.SpawnAreas`))
  (bind _box (`/Game/Blueprints/SpawnPoint.Box` (`|GetArrayItem` _spawnareas (`KismetMathLibrary.RandomInteger` (`KismetArrayLibrary.Array_Length` _spawnareas)))))
  (bind (_returnvalue_x _returnvalue_y _returnvalue_z) (`KismetMathLibrary.BreakVector` (`SceneComponent.K2_GetComponentLocation` _box)))
  (bind (_origin _boxextent) (`KismetSystemLibrary.GetComponentBounds` _box))
  (return (+ (`KismetMathLibrary.MakeVector` _returnvalue_x _returnvalue_y _returnvalue_z) (`KismetMathLibrary.MakeVector` (`KismetMathLibrary.RandomFloatInRange` (* (.x _boxextent) -1.0) (.x _boxextent)) (`KismetMathLibrary.RandomFloatInRange` (* (.y _boxextent) -1.0) (.y _boxextent))))))

(fn `SpawnWave`
  (locals (Basics :type Integer) (Bursters :type Integer) (Speeders :type Integer) (Tanks :type Integer) (Bosses :type Integer))
  (bind _difficultypoints (`self.DifficultyPoints`))
  (bind _returnvalue (`KismetMathLibrary.FFloor` (/ _difficultypoints 4.0)))
  (bind _returnvalue_2 (`KismetMathLibrary.FFloor` (/ _difficultypoints 5000.0)))
  (bind _returnvalue_3 (`KismetMathLibrary.FFloor` (/ _difficultypoints 2500.0)))
  (bind _returnvalue_4 (`KismetMathLibrary.FFloor` (/ _difficultypoints 500.0)))
  (bind _returnvalue_5 (`KismetMathLibrary.FFloor` (/ _difficultypoints 50.0)))
  ;[1 1 1] Calculate Enemies
  (`/Engine/EditorBlueprintResources/StandardMacros.IncrementInt` (`self.CurrentWave`)
    (:`  `
      (set `local.Bosses` _returnvalue_2)
      (set `self.DifficultyPoints` (- _difficultypoints (* _returnvalue_2 5000)))
      (set `local.Tanks` _returnvalue_3)
      (set `self.DifficultyPoints` (- _difficultypoints (* _returnvalue_3 2500)))
      (set `local.Speeders` _returnvalue_4)
      (set `self.DifficultyPoints` (- _difficultypoints (* _returnvalue_4 500)))
      (set `local.Bursters` _returnvalue_5)
      (set `self.DifficultyPoints` (- _difficultypoints (* _returnvalue_5 50)))
      (set `local.Basics` _returnvalue)
      (set `self.DifficultyPoints` (- _difficultypoints (* _returnvalue 4)))
      ;[1 1 1] Spawn Enemies
      (`|ExecutionSequence`
        (:`then_0`
          (for _ (range 1 (+ (`local.Basics`) 1))
            (bind _returnvalue_6 (`|SpawnActorFromClass` "/Game/Blueprints/Enemies/EnemyBasic.EnemyBasic_C" (`KismetMathLibrary.MakeTransform` (`self.GetRandomSpawn`)) "AlwaysSpawn" "MultiplyWithRoot" null null null))
            (`|SpawnActorFromClass` "/Game/Blueprints/ControllerManager.ControllerManager_C" (`KismetMathLibrary.MakeTransform` (0.0 0.0 0.0)) "Undefined" "MultiplyWithRoot" null _returnvalue_6 self 4.0 (`|MakeArray` (make `/Game/Blueprints/WeightedItem` null 5.0) (make `/Game/Blueprints/WeightedItem` "/Game/Blueprints/PickUps/BP_AmmoPickUp.BP_AmmoPickUp_C" 1.0) :!type "/Game/Blueprints/WeightedItem Structure") null)
            (`/Engine/EditorBlueprintResources/StandardMacros.IncrementInt` (`self.EnemiesLeft`))))
        (:`then_1`
          (for _ (range 1 (+ (`local.Bursters`) 1))
            (bind _returnvalue_7 (`|SpawnActorFromClass` "/Game/Blueprints/Enemies/EnemyBurster.EnemyBurster_C" (`KismetMathLibrary.MakeTransform` (`self.GetRandomSpawn`)) "AlwaysSpawn" "MultiplyWithRoot" null null null))
            (`|SpawnActorFromClass` "/Game/Blueprints/ControllerManager.ControllerManager_C" (`KismetMathLibrary.MakeTransform` (0.0 0.0 0.0)) "Undefined" "MultiplyWithRoot" null _returnvalue_7 self 50.0 (`|MakeArray` (make `/Game/Blueprints/WeightedItem` null 30.0) (make `/Game/Blueprints/WeightedItem` "/Game/Blueprints/PickUps/BP_HealPickUp.BP_HealPickUp_C" 8.0) (make `/Game/Blueprints/WeightedItem` "/Game/Blueprints/Weapons/BP_Shotgun.BP_Shotgun_C" 1.0) :!type "/Game/Blueprints/WeightedItem Structure") null)
            (`/Engine/EditorBlueprintResources/StandardMacros.IncrementInt` (`self.EnemiesLeft`))))
        (:`then_2`
          (for _ (range 1 (+ (`local.Speeders`) 1))
            (bind _returnvalue_8 (`|SpawnActorFromClass` "/Game/Blueprints/Enemies/EnemySpeeder.EnemySpeeder_C" (`KismetMathLibrary.MakeTransform` (`self.GetRandomSpawn`)) "AlwaysSpawn" "MultiplyWithRoot" null null null))
            (`|SpawnActorFromClass` "/Game/Blueprints/ControllerManager.ControllerManager_C" (`KismetMathLibrary.MakeTransform` (0.0 0.0 0.0)) "Undefined" "MultiplyWithRoot" null _returnvalue_8 self 50.0 (`|MakeArray` (make `/Game/Blueprints/WeightedItem` null 100.0) (make `/Game/Blueprints/WeightedItem` "/Game/Blueprints/PickUps/BP_HealPickUp.BP_HealPickUp_C" 60.0) (make `/Game/Blueprints/WeightedItem` "/Game/Blueprints/Weapons/BP_AR.BP_AR_C" 40.0) :!type "/Game/Blueprints/WeightedItem Structure") null)
            (`/Engine/EditorBlueprintResources/StandardMacros.IncrementInt` (`self.EnemiesLeft`))))
        (:`then_3`
          (for _ (range 1 (+ (`local.Tanks`) 1))
            (bind _returnvalue_9 (`|SpawnActorFromClass` "/Game/Blueprints/Enemies/EnemyTank.EnemyTank_C" (`KismetMathLibrary.MakeTransform` (`self.GetRandomSpawn`)) "AlwaysSpawn" "MultiplyWithRoot" null null null))
            (`|SpawnActorFromClass` "/Game/Blueprints/ControllerManager.ControllerManager_C" (`KismetMathLibrary.MakeTransform` (0.0 0.0 0.0)) "Undefined" "MultiplyWithRoot" null _returnvalue_9 self 50.0 (`|MakeArray` (make `/Game/Blueprints/WeightedItem` "/Game/Blueprints/PickUps/BP_HealPickUp.BP_HealPickUp_C" 100.0) (make `/Game/Blueprints/WeightedItem` "/Game/Blueprints/PickUps/BP_AmmoPickUp.BP_AmmoPickUp_C" 60.0) (make `/Game/Blueprints/WeightedItem` "/Game/Blueprints/Weapons/BP_AR.BP_AR_C" 40.0) :!type "/Game/Blueprints/WeightedItem Structure") null)
            (`/Engine/EditorBlueprintResources/StandardMacros.IncrementInt` (`self.EnemiesLeft`))))
        (:`then_4`
          (for _ (range 1 (+ (`local.Bosses`) 1))
            (bind _returnvalue_10 (`|SpawnActorFromClass` "/Game/Blueprints/Enemies/EnemyBoss.EnemyBoss_C" (`KismetMathLibrary.MakeTransform` (`self.GetRandomSpawn`)) "AlwaysSpawn" "MultiplyWithRoot" null null null))
            (`|SpawnActorFromClass` "/Game/Blueprints/ControllerManager.ControllerManager_C" (`KismetMathLibrary.MakeTransform` (0.0 0.0 0.0)) "Undefined" "MultiplyWithRoot" null _returnvalue_10 self 50.0 (`|MakeArray` (make `/Game/Blueprints/WeightedItem` "/Game/Blueprints/PickUps/BP_HealPickUp.BP_HealPickUp_C" 100.0) :!type "/Game/Blueprints/WeightedItem Structure") null)
            (`/Engine/EditorBlueprintResources/StandardMacros.IncrementInt` (`self.EnemiesLeft`))))))))

(fn `UserConstructionScript`)